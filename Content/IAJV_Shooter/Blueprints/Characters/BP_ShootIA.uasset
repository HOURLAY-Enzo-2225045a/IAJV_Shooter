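; BP_ShootIA is a shooter character Blueprint that handles aim-down-sights input and its own health bar.
; On BeginPlay it creates the Aim crosshair widget and registers itself as owner of the HealthBar in its HealthWidget component.
; Holding Aiming shows the crosshair, slows walking and stops orienting rotation to movement, while a timeline lerps the camera boom closer.
; Releasing hides the crosshair, restores speed and movement-based rotation, and reverses the timeline.
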(event EventBeginPlay
  (bind _returnvalue (UserInterface|CreateWidget "/Game/UI/Aim.Aim_C"))
  (Variables|Default|SetCrosshair _returnvalue)
  (bind _ashealth_bar (Utilities|Casting|CastToHealthBar (UserInterface|GetUserWidgetObject (Variables|Default|GetHealthWidget))))
  (Variables|/Game/UI/HealthBar.HealthBar_C|SetHealthBarOwner _ashealth_bar self))

(event Collision|EventActorBeginOverlap
  (params (OtherActor :type Actor%20Object%20Reference)))

(event EventTick
  (params (DeltaSeconds :type Float%20%28single-precision%29)))

(event Input|ActionEvents|InputActionAiming
  (params (Key :type Key%20Structure :default "None"))
  (bind _charactermovement (Variables|Character|GetCharacterMovement))
  (bind _crosshair (Variables|Default|GetCrosshair))
  (bind _charactermovement_2 (Variables|Character|GetCharacterMovement))
  (:Pressed
    (UserInterface|Viewport|AddtoViewport _crosshair 0)
    (Variables|/Script/Engine.CharacterMovementComponent|SetMaxWalkSpeed _charactermovement_2 2e+02)
    (Variables|/Script/Engine.CharacterMovementComponent|SetbOrientRotationToMovement _charactermovement false)
    (Variables|/Script/Engine.CharacterMovementComponent|SetbUseControllerDesiredRotation _charactermovement true)
    (bind _newtrack_0 (Timeline|Aiming Play)
      (:Update
        (Variables|/Script/Engine.SpringArmComponent|SetTargetArmLength (Variables|Default|GetCameraBoom) (Math|Float|Lerp 4e+02 2e+02 _newtrack_0)))))
  (:Released
    (Widget|RemovefromParent _crosshair)
    (Variables|/Script/Engine.CharacterMovementComponent|SetMaxWalkSpeed _charactermovement_2 5e+02)
    (Variables|/Script/Engine.CharacterMovementComponent|SetbOrientRotationToMovement _charactermovement true)
    (Variables|/Script/Engine.CharacterMovementComponent|SetbUseControllerDesiredRotation _charactermovement true)
    (Timeline|Aiming Reverse)))

(fn ConstructionScript)